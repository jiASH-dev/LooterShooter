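; BP_Weapon is a weapon actor that fires projectiles and ejects physics-driven shell casings, with settable projectile class, shell class, weight and wearing type.
; DoFire rate-limits shots with a short delay gate, and ExecuteFire spawns a projectile at the arrow component.
; Shells are pooled: new ones spawn up to a maximum, then existing ones are relaunched round-robin.
; EndFire starts a timer that destroys the pool, which renewed firing cancels.
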(event Custom|DoFire
  (Utilities|Time|ClearTimerbyFunctionName 0 "ClearShellsPool")
  (if (Variables|Default|GetIsWeaponReadyToFire)
    (CallFunction|ExecuteFire)
    (Variables|Default|SetIsWeaponReadyToFire false)
    (Utilities|FlowControl|Delay 0.1)
    (Variables|Default|SetIsWeaponReadyToFire true)))

(event EventBeginPlay)

(event Collision|EventActorBeginOverlap
  (params (OtherActor :type Actor%20Object%20Reference)))

(event EventTick
  (params (DeltaSeconds :type Float%20%28single-precision%29)))

(fn ConstructionScript)

(fn GetWeight
  (return (Variables|WeaponSpecs|GetWeight)))

(fn SetWeight
  (params (Weight :type Float%20%28double-precision%29))
  (Variables|WeaponSpecs|SetWeight Weight))

(fn SetProjectileClass
  (params (ProjectileClass :type BP%20Projectile%20Class%20Reference))
  (Variables|Default|SetProjectileClass ProjectileClass))

(fn SetShellClass
  (params (ShellClass :type BP%20Shell%20Class%20Reference))
  (Variables|Default|SetShellClass ShellClass))

(fn SetWearingType
  (params (WearingType :type E_WeaponWearingType%20Enum :default "NewEnumerator0"))
  (Variables|Default|SetWearingType WearingType))

(fn GetWearingType
  (return (Variables|Default|GetWearingType)))

(fn SpawnWeaponShell
  (bind _returnvalue (Game|SpawnActorfromClass (Variables|Default|GetShellClass) (Math|Transform|MakeTransform (Transformation|GetWorldLocation (Variables|Default|GetShellSpawnPlaceSceneComponent))) "Undefined" "MultiplyWithRoot" 0 0))
  (CallFunction|SetupShellLocationandPhysics _returnvalue)
  (return _returnvalue))

(fn SpawnWeaponProjectile
  (Game|SpawnActorfromClass (Variables|Default|GetProjectileClass) (Transformation|GetWorldTransform (Variables|Default|GetProjectileSpawnPlaceArrow)) "Undefined" "MultiplyWithRoot" 0 0))

(fn SetupShellLocationandPhysics
  (params (Shell :type BP%20Shell%20Object%20Reference))
  (bind _shellstaticmeshcomponent (Variables|/Game/Blueprints/Ammo/BP_Shell.BP_Shell_C|GetShellStaticMeshComponent Shell))
  (bind _returnvalue (Transformation|GetWorldRotation _shellstaticmeshcomponent))
  (bind _returnvalue_2 (Math|Vector|GetRightVector _returnvalue))
  (bind (_x _y _z) (Math|Vector|BreakVector _returnvalue_2))
  (Transformation|SetWorldLocation _shellstaticmeshcomponent (Transformation|GetWorldLocation (Variables|Default|GetShellSpawnPlaceSceneComponent)) false false)
  (Physics|SetPhysicsLinearVelocity _shellstaticmeshcomponent (Math|Vector|MakeVector (* _x 2e+02) (* _y 2e+02) (+ _z 1.5e+02)) false "None"))

(fn ExecuteFire
  (if (< (Utilities|Array|Length (Variables|Default|GetShellsPool)) (Variables|Default|GetMaxShellsNumber))
    (CallFunction|SpawnWeaponProjectile)
    (bind _shell (CallFunction|SpawnWeaponShell))
    (Utilities|Array|Add (Variables|Default|GetShellsPool) _shell)
    (else
      (if (== (Variables|Default|GetCurrentShellIndex) (Variables|Default|GetMaxShellsNumber))
        (Variables|Default|SetCurrentShellIndex 0))
      (CallFunction|SpawnWeaponProjectile)
      (CallFunction|SetupShellLocationandPhysics (Utilities|Array|Get(acopy) (Variables|Default|GetShellsPool) (Variables|Default|GetCurrentShellIndex)))
      (Math|Integer|IncrementInt (Variables|Default|GetCurrentShellIndex)))))

(fn GetShellsPool
  (return (Variables|Default|GetShellsPool)))

(fn EndFire
  (Utilities|Time|SetTimerbyFunctionName 0 "ClearShellsPool" 2.0))

(fn ClearShellsPool
  (bind _shellspool (Variables|Default|GetShellsPool))
  (for _array_element _shellspool
    (Actor|DestroyActor _array_element))
  (Utilities|Array|Clear _shellspool))