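; BP_AK-47 is an AK-47 weapon Blueprint that only configures behavior inherited from its parent class.
; Its construction script runs the parent's, then sets the 5.45 projectile and shell classes, a wearing type and the weapon's weight.
; The event graph holds only disabled placeholder events, so it adds no runtime logic of its own.
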(event EventBeginPlay
  (|CallParentFunction) ; This node is disabled and will not be called.\nDrag off pins to build functionality.
)

(event Collision|EventActorBeginOverlap
  (params (OtherActor :type Actor%20Object%20Reference))
  (|CallParentFunction OtherActor) ; This node is disabled and will not be called.\nDrag off pins to build functionality.
)

(event EventTick
  (params (DeltaSeconds :type Float%20%28single-precision%29))
  (|CallParentFunction DeltaSeconds) ; This node is disabled and will not be called.\nDrag off pins to build functionality.
)

(fn ConstructionScript
  (|CallParentFunction)
  (CallFunction|SetProjectileClass "/Game/Blueprints/Ammo/BP_Projectile545.BP_Projectile545_C")
  (CallFunction|SetShellClass "/Game/Blueprints/Ammo/BP_Shell545.BP_Shell545_C")
  (CallFunction|SetWearingType "NewEnumerator0")
  (CallFunction|SetWeight 3e+01))