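; BP_Gunner is a player character with walking, running, crouching, sliding, aiming and shooting.
; Slide duration derives from speed, floor friction and gravity; a looping timer stands the character up once overhead collision clears.
; Traced pickups fill back or side slots as single or modificated weapons, which drive switching, aim socket attachment and timer-based automatic fire.
; SetupWeapon's attach and weight logic is disconnected, so it never runs.
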(event EventTick
  (params (DeltaSeconds :type Float%20%28single-precision%29)))

(event Input|ActionEvents|InputActionSliding
  (params (Key :type Key%20Structure))
  (:Pressed
    (if (Math|Boolean|ANDBoolean (>= (Class|KismetAnimationLibrary|CalculateDirection (Variables|/Script/Engine.MovementComponent|GetVelocity (Variables|Character|GetCharacterMovement)) (Transformation|GetActorRotation)) -5e+01) (<= (Class|KismetAnimationLibrary|CalculateDirection (Variables|/Script/Engine.MovementComponent|GetVelocity (Variables|Character|GetCharacterMovement)) (Transformation|GetActorRotation)) 5e+01) (== (Variables|Default|GetIsCharacterSliding) false) (> (Math|Vector|VectorLength (Variables|/Script/Engine.MovementComponent|GetVelocity (Variables|Character|GetCharacterMovement))) 8e+02))
      (Variables|Default|SetIsCharacterSliding true)
      (Variables|Default|SetCharacterState "NewEnumerator1")
      (Variables|Default|SetInitialVelocity (Variables|/Script/Engine.MovementComponent|GetVelocity (Variables|Character|GetCharacterMovement)))
      (bind _slidingdirection (CallFunction|CalculateSlidingDirection))
      (bind _slidinganimationrate (CallFunction|CalculateSlidingAnimationRate _slidingdirection))
      (Components|Timeline|SetTimelineLength (Variables|Default|GetSlide) _slidingdirection)
      (Animation|PlayAnimMontage "/Game/Animations/AM_Sliding.AM_Sliding" _slidinganimationrate "None")
      (bind _slideinterpdeltatime (Timeline|Slide PlayFromStart)
        (:Update
          (Variables|/Script/Engine.MovementComponent|SetVelocity (Variables|Character|GetCharacterMovement) (Math|Interpolation|VInterpTo (Variables|Default|GetInitialVelocity) "0, 0, 0" _slideinterpdeltatime 0.5)))
        (:Finished
          (Utilities|FlowControl|Delay 0.2)
          (Variables|Default|SetIsCharacterSliding false)
          (Variables|Default|SetCharacterState "NewEnumerator0"))))))

(event Input|ActionEvents|InputActionCrouch
  (params (Key :type Key%20Structure))
  (bind _mesh (Variables|Character|GetMesh))
  (bind _bodycollisioncomponent (Variables|Default|GetBodyCollisionComponent))
  (bind _capsulecomponent (Variables|Default|GetCapsuleComponent))
  (bind _relativelocation (Variables|/Script/Engine.SceneComponent|GetRelativeLocation _mesh))
  (bind _relativelocation_2 (Variables|/Script/Engine.SceneComponent|GetRelativeLocation _bodycollisioncomponent))
  (bind (_x _y _z) (Math|Vector|BreakVector _relativelocation))
  (bind (_x_2 _y_2 _z_2) (Math|Vector|BreakVector _relativelocation_2))
  (:Pressed
    (if (not (Variables|Default|GetIsCharacterCrouching))
      (Components|Capsule|SetCapsuleHalfHeight _capsulecomponent (/ (Variables|/Script/Engine.CapsuleComponent|GetCapsuleHalfHeight _capsulecomponent) (Variables|Default|GetCrouchHeightDelta)) true)
      (Transformation|SetRelativeLocation _bodycollisioncomponent (Math|Vector|MakeVector _x_2 _y_2 (+ _z_2 (Variables|/Script/Engine.CapsuleComponent|GetCapsuleHalfHeight (Variables|Default|GetCapsuleComponent)))) false false)
      (Transformation|SetRelativeLocation _mesh (Math|Vector|MakeVector _x _y (/ _z (Variables|Default|GetCrouchHeightDelta))) false false)
      (Variables|/Script/Engine.CharacterMovementComponent|SetMaxWalkSpeed (Variables|Character|GetCharacterMovement) (- (Variables|Default|GetCrouchingSpeed) (Variables|Default|GetWeaponWeight)))
      (Variables|Default|SetIsCharacterCrouching true)))
  (:Released
    (if (Variables|Default|GetIsCharacterCrouching)
      (Utilities|Time|SetTimerbyFunctionName 0 "TryToRaiseCharacter" 0.01 true))))

(event Input|ActionEvents|InputActionTakeAim
  (params (Key :type Key%20Structure))
  (bind _spline (Variables|Default|GetSpline))
  (:Pressed
    (if (and (<= (Math|Vector|VectorLength (Variables|/Script/Engine.MovementComponent|GetVelocity (Variables|Character|GetCharacterMovement))) (Variables|Default|GetWalkingSpeed)) (Variables|Default|GetIsCharacterWithWeapon))
      (Variables|Default|SetCharacterState "NewEnumerator2")
      (switch Utilities|FlowControl|Switch|SwitchonE_WeaponTypeInHands (Variables|Default|GetCurrentWeaponTypeInHand)
        (:NewEnumerator1
          (Transformation|AttachComponentToComponent (Variables|Default|GetCurrentSingleWeaponInHands) (Variables|Character|GetMesh) "LeftHandSocketAiming" "SnapToTarget" "SnapToTarget" "SnapToTarget" true)
          (bind _aimdeltatime (Timeline|Aim PlayFromStart)
            (:Update
              (Transformation|SetRelativeLocation (Variables|Default|GetCamera) (Math|Interpolation|VInterpTo (Spline|GetLocationatSplinePoint _spline 0 "Local") (Spline|GetLocationatSplinePoint _spline 1 "Local") _aimdeltatime 1.0) false false))))
        (:NewEnumerator2
          (Transformation|AttachComponentToComponent (Variables|Default|GetCurrentModificatedWeaponInHands) (Variables|Character|GetMesh) "LeftHandSocketAiming" "SnapToTarget" "SnapToTarget" "SnapToTarget" true)
          (Timeline|Aim PlayFromStart)))))
  (:Released
    (Variables|Default|SetCharacterState "NewEnumerator0")
    (switch Utilities|FlowControl|Switch|SwitchonE_WeaponTypeInHands (Variables|Default|GetCurrentWeaponTypeInHand)
      (:NewEnumerator1
        (Transformation|AttachComponentToComponent (Variables|Default|GetCurrentSingleWeaponInHands) (Variables|Character|GetMesh) "LeftHandSocketIdle" "SnapToTarget" "SnapToTarget" "SnapToTarget" true)
        (Timeline|Aim Reverse))
      (:NewEnumerator2
        (Transformation|AttachComponentToComponent (Variables|Default|GetCurrentModificatedWeaponInHands) (Variables|Character|GetMesh) "LeftHandSocketIdle" "SnapToTarget" "SnapToTarget" "SnapToTarget" true)
        (Timeline|Aim Reverse)))))

(event Input|ActionEvents|InputActionTryToPickupWeapon
  (params (Key :type Key%20Structure))
  (bind _returnvalue (Transformation|GetActorLocation))
  (bind _weapontypesplaces (Variables|Default|GetWeaponTypesPlaces))
  (bind _weapontypesplaces_2 (Variables|Default|GetWeaponTypesPlaces))
  (:Pressed
    (bind (_outhit _returnvalue_2) (Collision|LineTraceByChannel _returnvalue (+ _returnvalue "200.000000,0.000000,0.000000") "TraceTypeQuery3" false 0 "None"))
    (if _returnvalue_2
      (bind _asbp_modes_weapon (Utilities|Casting|CastToBP_ModificatedWeapon (.HitActor (Collision|BreakHitResult _outhit)))
        (:then
          (switch Utilities|FlowControl|Switch|SwitchonE_WeaponWearingType (Default|GetWearingType _asbp_modes_weapon)
            (:NewEnumerator0
              (Utilities|Map|Add _weapontypesplaces_2 "NewEnumerator1" "NewEnumerator1")
              (bind _output_get (Variables|Default|SetModificatedWeaponOnTheBack _asbp_modes_weapon))
              (CallFunction|SetupWeapon _output_get))
            (:NewEnumerator1
              (Utilities|Map|Add _weapontypesplaces_2 "NewEnumerator2" "NewEnumerator1")
              (bind _output_get_2 (Variables|Default|SetModificatedWeaponOnTheSide _asbp_modes_weapon))
              (CallFunction|SetupWeapon _output_get_2))))
        (:CastFailed
          (bind _asbp_weapon (Utilities|Casting|CastToBP_Weapon (.HitActor (Collision|BreakHitResult _outhit))))
          (switch Utilities|FlowControl|Switch|SwitchonE_WeaponWearingType (Default|GetWearingType _asbp_weapon)
            (:NewEnumerator0
              (Utilities|Map|Add _weapontypesplaces "NewEnumerator1" "NewEnumerator0")
              (bind _output_get_3 (Variables|Default|SetSingleWeaponOnTheBack _asbp_weapon))
              (CallFunction|SetupWeapon _output_get_3))
            (:NewEnumerator1
              (Utilities|Map|Add _weapontypesplaces "NewEnumerator2" "NewEnumerator0")
              (bind _output_get_4 (Variables|Default|SetSingleWeaponOnTheSide _asbp_weapon))
              (CallFunction|SetupWeapon _output_get_4))))))))

(event Input|ActionEvents|InputActionChangeWeaponMode
  (params (Key :type Key%20Structure))
  (:Pressed
    (switch Utilities|FlowControl|Switch|SwitchonE_WeaponTypeInHands (Variables|Default|GetCurrentWeaponTypeInHand)
      (:NewEnumerator2
        (Default|ChangeCurrentShootingMode (Variables|Default|GetCurrentModificatedWeaponInHands))))))

(event Input|ActionEvents|InputActionChangeWeapon
  (params (Key :type Key%20Structure))
  (:Pressed
    (switch Utilities|FlowControl|Switch|SwitchonE_WeaponPlace (Variables|Default|GetCurrentWeaponInHandFromPlace)
      (:NewEnumerator1
        (CallFunction|ChangeWeaponbytheSidePlace)
        (Variables|Default|SetIsCharacterWithWeapon true :!label _label))
      (:NewEnumerator2
        (CallFunction|ChangeWeaponbytheBackPlace)
        (goto _label))
      (:NewEnumerator3
        (if (.ReturnValue (Utilities|Map|Find (Variables|Default|GetWeaponTypesPlaces) "NewEnumerator2"))
          (CallFunction|ChangeWeaponbytheSidePlace)
          (goto _label)
          (elif (.ReturnValue (Utilities|Map|Find (Variables|Default|GetWeaponTypesPlaces) "NewEnumerator1"))
            (CallFunction|ChangeWeaponbytheBackPlace)
            (goto _label)))))))

(event Input|AxisEvents|InputAxisMoveVertical
  (params (AxisValue :type Float%20%28single-precision%29))
  (if (not (Variables|Default|GetIsCharacterSliding))
    (Pawn|Input|AddMovementInput (Math|Vector|GetForwardVector (Transformation|GetActorRotation)) AxisValue false)))

(event Input|AxisEvents|InputAxisMoveHorizontal
  (params (AxisValue :type Float%20%28single-precision%29))
  (if (not (Variables|Default|GetIsCharacterSliding))
    (Pawn|Input|AddMovementInput (Math|Vector|GetRightVector (Transformation|GetActorRotation)) AxisValue false)))

(event Input|AxisEvents|InputAxisRun
  (params (AxisValue :type Float%20%28single-precision%29))
  (bind _charactermovement (Variables|Character|GetCharacterMovement))
  (if (== (Variables|Default|GetIsCharacterCrouching) false)
    (if (and (> AxisValue 0.0) (> (.X (Math|Vector|BreakVector (Variables|/Script/Engine.MovementComponent|GetVelocity (Variables|Character|GetCharacterMovement)))) 0.0))
      (Variables|/Script/Engine.CharacterMovementComponent|SetMaxWalkSpeed _charactermovement (- (Variables|Default|GetRunningSpeed) (Variables|Default|GetWeaponWeight)))
      (else
        (Variables|/Script/Engine.CharacterMovementComponent|SetMaxWalkSpeed _charactermovement (- (Variables|Default|GetWalkingSpeed) (Variables|Default|GetWeaponWeight)))))))

(event Input|MouseEvents|LeftMouseButton
  (params (Key :type Key%20Structure))
  ;[1 0 0.2264] Переименовать
  (:Pressed
    (switch Utilities|FlowControl|Switch|SwitchonE_WeaponTypeInHands (Variables|Default|GetCurrentWeaponTypeInHand)
      (:NewEnumerator1
        (Default|DoFire (Variables|Default|GetCurrentSingleWeaponInHands)))
      (:NewEnumerator2
        (Variables|Default|SetIsAutomaticShootingEnded false)
        (switch Utilities|FlowControl|Switch|SwitchonE_WeaponShootingMode (Default|GetCurrentShootingMode (Variables|Default|GetCurrentModificatedWeaponInHands))
          (:NewEnumerator0
            (Default|DoFire (Variables|Default|GetCurrentModificatedWeaponInHands)))
          (:NewEnumerator1
            (Utilities|Time|SetTimerbyFunctionName 0 "DoAutomaticShooting" 0.1 true))))))
  (:Released
    (switch Utilities|FlowControl|Switch|SwitchonE_WeaponTypeInHands (Variables|Default|GetCurrentWeaponTypeInHand)
      (:NewEnumerator2
        (Variables|Default|SetIsAutomaticShootingEnded true)))))

(fn ConstructionScript)

(fn GetIsCharacterwithWeapon
  (return (Variables|Default|GetIsCharacterWithWeapon)))

(fn GetIsCharacterCrouching
  (return (Variables|Default|GetIsCharacterCrouching)))

(fn TrytoRaiseCharacter
  (bind _bodycollisioncomponent (Variables|Default|GetBodyCollisionComponent))
  (bind _capsulecomponent (Variables|Default|GetCapsuleComponent))
  (bind _mesh (Variables|Character|GetMesh))
  (bind _relativelocation (Variables|/Script/Engine.SceneComponent|GetRelativeLocation _mesh))
  (bind _relativelocation_2 (Variables|/Script/Engine.SceneComponent|GetRelativeLocation _bodycollisioncomponent))
  (bind (_x _y _z) (Math|Vector|BreakVector _relativelocation))
  (bind (_x_2 _y_2 _z_2) (Math|Vector|BreakVector _relativelocation_2))
  (if (== (Utilities|Array|Length (Collision|GetOverlappingActors (Variables|Default|GetBodyCollisionComponent) "/Script/Engine.Actor" :!class /Script/Engine.PrimitiveComponent)) 0)
    (Transformation|SetRelativeLocation _bodycollisioncomponent (Math|Vector|MakeVector _x_2 _y_2 (- _z_2 (Variables|/Script/Engine.CapsuleComponent|GetCapsuleHalfHeight (Variables|Default|GetCapsuleComponent)))) false false)
    (Components|Capsule|SetCapsuleHalfHeight _capsulecomponent (* (Variables|/Script/Engine.CapsuleComponent|GetCapsuleHalfHeight _capsulecomponent) (Variables|Default|GetCrouchHeightDelta)) true)
    (Transformation|SetRelativeLocation _mesh (Math|Vector|MakeVector _x _y (* _z (Variables|Default|GetCrouchHeightDelta))) false false)
    (Variables|Default|SetIsCharacterCrouching false)
    (Variables|/Script/Engine.CharacterMovementComponent|SetMaxWalkSpeed (Variables|Character|GetCharacterMovement) (- (Variables|Default|GetWalkingSpeed) (Variables|Default|GetWeaponWeight)))
    (Utilities|Time|ClearTimerbyFunctionName 0 "TryToRaiseCharacter")))

(fn GetCharacterState
  (return (Variables|Default|GetCharacterState)))

(fn DoAutomaticShooting
  (if (Variables|Default|GetIsAutomaticShootingEnded)
    (Default|DoFire (Variables|Default|GetCurrentModificatedWeaponInHands))
    (Utilities|Time|ClearTimerbyFunctionName 0 "DoAutomaticShooting")
    (else
      (Default|DoFire (Variables|Default|GetCurrentModificatedWeaponInHands)))))

(fn SetupWeapon
  (params (Weapon :type BP%20Weapon%20Object%20Reference))
  ;[1 0.005695 0] Не правильно работает привязка
)

(fn CalculateSlidingDirection
  (bind _returnvalue (Transformation|GetActorLocation))
  (bind _outhit (Collision|LineTraceByChannel _returnvalue (- _returnvalue "0.000000,0.000000,100.000000") "TraceTypeQuery1" false 0 "None"))
  (return (/ (/ (Math|Vector|VectorLength (Variables|Default|GetInitialVelocity)) (Variables|/Script/PhysicsCore.PhysicalMaterial|GetFriction (.PhysMat (Collision|BreakHitResult _outhit)))) (* (Components|Movement|GetGravityZ (Variables|Character|GetCharacterMovement)) -1.0))))

(fn CalculateSlidingAnimationRate
  (params (SlidingDirection :type Float%20%28double-precision%29))
  (return (+ (/ (/ 37.0 (/ 1.0 (Utilities|Time|GetWorldDeltaSeconds))) SlidingDirection) 0.1)))

(fn ChangeWeaponbytheSidePlace
  (bind _weapontypesplaces (Variables|Default|GetWeaponTypesPlaces))
  (bind (_value _returnvalue) (Utilities|Map|Find _weapontypesplaces "NewEnumerator2"))
  (if _returnvalue
    (switch Utilities|FlowControl|Switch|SwitchonE_WeaponType _value
      (:NewEnumerator0
        (Variables|Default|SetCurrentSingleWeaponInHands (Variables|Default|GetSingleWeaponOnTheSide))
        (Variables|Default|SetCurrentWeaponTypeInHand "NewEnumerator1"))
      (:NewEnumerator1
        (Variables|Default|SetCurrentModificatedWeaponInHands (Variables|Default|GetModificatedWeaponOnTheSide))
        (Variables|Default|SetCurrentWeaponTypeInHand "NewEnumerator2")))
    (Variables|Default|SetCurrentWeaponInHandFromPlace "NewEnumerator2")))

(fn ChangeWeaponbytheBackPlace
  (bind _weapontypesplaces (Variables|Default|GetWeaponTypesPlaces))
  (bind (_value _returnvalue) (Utilities|Map|Find _weapontypesplaces "NewEnumerator1"))
  (if _returnvalue
    (switch Utilities|FlowControl|Switch|SwitchonE_WeaponType _value
      (:NewEnumerator0
        (Variables|Default|SetCurrentSingleWeaponInHands (Variables|Default|GetSingleWeaponOnTheBack))
        (Variables|Default|SetCurrentWeaponTypeInHand "NewEnumerator1"))
      (:NewEnumerator1
        (Variables|Default|SetCurrentModificatedWeaponInHands (Variables|Default|GetModificatedWeaponOnTheBack))
        (Variables|Default|SetCurrentWeaponTypeInHand "NewEnumerator2")))
    (Variables|Default|SetCurrentWeaponInHandFromPlace "NewEnumerator1")))